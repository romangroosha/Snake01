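; Berry pickup actor for a snake game, consumed when MouseSnake_BP overlaps it.
; On overlap it sends a Berryable interface message to the snake's last body segment, then destroys itself.
; BeginPlay caches snake, character and game mode references and registers with the game mode's move ticker, though its handler is empty.
; A similar branch for the turn-based Character_BP snake is disconnected.
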(event `MoveTicker_Event`)

(event `self.ReceiveBeginPlay`
  (`self.Set_MouseSnakeBP_ref`)
  (`self.Character_BP_ref`)
  (`self.GameModeBase_BP_ref`)
  (add `/Game/BP/GameModeBase_BP.MoveTicker` (`self.GameModeBase_BP`) (`|CreateDelegate` :!event `MoveTicker_Event`)))

(event `self.ReceiveActorBeginOverlap`
  (params (OtherActor :type "Actor Object Reference"))
  (if (== (`GameplayStatics.GetObjectClass` OtherActor) "/Game/BP/MouseSnake_BP.MouseSnake_BP_C")
    (message `/Game/BP/Berryable_INT.Berryable_Interface` (`|GetArrayItem` (`/Game/BP/MouseSnake_BP.SnakeBodyArr` (`self.MouseSnakeBP_ref`)) (`KismetArrayLibrary.Array_LastIndex` (`/Game/BP/MouseSnake_BP.SnakeBodyArr` (`self.MouseSnakeBP_ref`)))))
    (`self.K2_DestroyActor`)))

(fn `Character_BP_ref`
  (`/Engine/EditorBlueprintResources/StandardMacros.IsValid` (`self.Character_BP`)
    (:`Is Not Valid`
      (bind _returnvalue (`GameplayStatics.GetActorOfClass` "/Game/BP/Old/Character_BP.Character_BP_C"))
      (set `self.Character_BP` _returnvalue))))

(fn `GameModeBase_BP_ref`
  (`/Engine/EditorBlueprintResources/StandardMacros.IsValid` (`self.GameModeBase_BP`)
    (:`Is Not Valid`
      (bind _returnvalue (`GameplayStatics.GetActorOfClass` "/Game/BP/GameModeBase_BP.GameModeBase_BP_C"))
      (set `self.GameModeBase_BP` _returnvalue))))

(fn `Set_MouseSnakeBP_ref`
  (`/Engine/EditorBlueprintResources/StandardMacros.IsValid` (`self.MouseSnakeBP_ref`)
    (:`Is Not Valid`
      (bind _returnvalue (`GameplayStatics.GetActorOfClass` "/Game/BP/MouseSnake_BP.MouseSnake_BP_C"))
      (set `self.MouseSnakeBP_ref` _returnvalue))))

(fn `UserConstructionScript`)