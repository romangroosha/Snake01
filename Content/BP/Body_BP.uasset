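; Body segment actor for a snake-style chain that follows its parent, either the Character_BP or another Body_BP.
; Each player-controller move command lerps its XY to the parent's stored previous location, using timelines scaled to the GameMode's tick rate.
; BerryableInterface opens a gate so the next finished move spawns one child segment at the vacated position and registers it in the character's BodyArr.
; On BeginPlay it scales up and displays its name's numeric suffix.
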(event `MoveTicker_Event`)

(event `self.ReceiveBeginPlay`
  (`self.Character_BP_ref`)
  (`self.GameModeBase_BP_ref`)
  (`self.PlayerController_BP_ref`)
  (add `/Game/BP/PlayerController_BP.MoveCommand_PC` (`self.PlayerController_BP`) (`|CreateDelegate` :!event `MoveCommand_PC`))
  (add `/Game/BP/GameModeBase_BP.MoveTicker` (`self.GameModeBase_BP`) (`|CreateDelegate` :!event `MoveTicker_Event`))
  (`self.CutStringShowNameDigit`)
  (`TimelineComponent.SetPlayRate` (`self.Timeline_0`) (/ 1.0 (`/Game/BP/GameModeBase_BP.TimeRate (in seconds)` (`self.GameModeBase_BP`))))
  (`TimelineComponent.SetPlayRate` (`self.Timeline_1`) (/ 1.0 (`/Game/BP/GameModeBase_BP.TimeRate (in seconds)` (`self.GameModeBase_BP`))))
  (`TimelineComponent.SetPlayRate` (`self.Timeline_Size`) (/ 1.0 (`/Game/BP/GameModeBase_BP.TimeRate (in seconds)` (`self.GameModeBase_BP`))))
  (bind (_direction _0_to_1) (`Timeline|Timeline_Size` :!via `PlayFromStart`)
    (:`Update`
      (`self.SetActorScale3D` (`KismetMathLibrary.VLerp` (0.1 0.1 0.1) (1.0 1.0 1.0) _0_to_1)))))

(event `MoveCommand_PC`
  (params (Location :type "Vector Structure") (Rotation :type "Rotator Structure"))
  (bind (_actorlocationba_x _actorlocationba_y) (`KismetMathLibrary.BreakVector` (`self.ActorLocationBA`)))
  (set `self.ActorLocationBA` (`self.K2_GetActorLocation`))
  (`self.WhoIsParentActor`
    (:`Chatacter_BP`
      (bind _ascharacter_bp (cast `/Game/BP/Character_BP` (`self.ParentAct`)))
      (bind (_direction _0_to_1) (`Timeline|Timeline_0` :!via `PlayFromStart`)
        (:`Update`
          (bind (_returnvalue_x _returnvalue_y) (`KismetMathLibrary.BreakVector` (`KismetMathLibrary.VLerp` (`self.ActorLocationBA`) (`/Game/BP/Character_BP.ActorLocationBA` _ascharacter_bp) _0_to_1)))
          (`self.K2_SetActorLocation` (`KismetMathLibrary.MakeVector` _returnvalue_x _returnvalue_y) false true))
        (:`Finished`
          (`/Engine/EditorBlueprintResources/StandardMacros.Gate` true :!label _label
            (:`Exit`
              (bind _returnvalue (`|SpawnActorFromClass` "Body_BP_C" (`KismetMathLibrary.MakeTransform` (`KismetMathLibrary.MakeVector` _actorlocationba_x _actorlocationba_y)) "Undefined" "OverrideRootScale" null null))
              (set `/Game/BP/Body_BP.ParentAct` self _returnvalue)
              (`KismetArrayLibrary.Array_Add` (`/Game/BP/Character_BP.BodyArr` (`self.Character_BP`)) _returnvalue)
              (goto _label :!via `Close`))))))
    (:`Body_BP`
      (bind _asbody_bp (cast `/Game/BP/Body_BP` (`self.ParentAct`)))
      (bind (_direction_2 _0_to_1_2) (`Timeline|Timeline_1` :!via `PlayFromStart`)
        (:`Update`
          (bind (_returnvalue_x_2 _returnvalue_y_2) (`KismetMathLibrary.BreakVector` (`KismetMathLibrary.VLerp` (`self.ActorLocationBA`) (`/Game/BP/Body_BP.ActorLocationBA` _asbody_bp) _0_to_1_2)))
          (`self.K2_SetActorLocation` (`KismetMathLibrary.MakeVector` _returnvalue_x_2 _returnvalue_y_2) false true))
        (:`Finished`
          (goto _label))))))

(event `/Game/BP/Berryable_INT.Berryable_Interface`
  (goto _label :!via `Open`))

(fn `Character_BP_ref`
  (`/Engine/EditorBlueprintResources/StandardMacros.IsValid` (`self.Character_BP`)
    (:`Is Not Valid`
      (bind _returnvalue (`GameplayStatics.GetActorOfClass` "/Game/BP/Character_BP.Character_BP_C"))
      (set `self.Character_BP` _returnvalue))))

(fn `CutStringShowNameDigit`
  (`TextRenderComponent.K2_SetText` (`self.TextRender`) (`KismetTextLibrary.Conv_StringToText` (`.RightS` (`KismetStringLibrary.Split` (`KismetSystemLibrary.GetObjectName` self) "_" "IgnoreCase" "FromEnd")))))

(fn `GameModeBase_BP_ref`
  (`/Engine/EditorBlueprintResources/StandardMacros.IsValid` (`self.GameModeBase_BP`)
    (:`Is Not Valid`
      (bind _returnvalue (`GameplayStatics.GetActorOfClass` "/Game/BP/GameModeBase_BP.GameModeBase_BP_C"))
      (set `self.GameModeBase_BP` _returnvalue))))

(fn `PlayerController_BP_ref`
  (`/Engine/EditorBlueprintResources/StandardMacros.IsValid` (`self.PlayerController_BP`)
    (:`Is Not Valid`
      (bind _returnvalue (`GameplayStatics.GetActorOfClass` "/Game/BP/PlayerController_BP.PlayerController_BP_C"))
      (set `self.PlayerController_BP` _returnvalue))))

(fn `UserConstructionScript`)