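; MouseSnake_BP is a snake head pawn that continually moves forward and steers toward the point under the mouse cursor.
; Tick sets yaw from an RInterpTo between the cursor look-at and current rotation, then adds half-strength forward input.
; BeginPlay spawns one MouseSnakeBody_BP, stores it in SnakeBodyArr and sets itself as its parent.
; Berry overlap handling is empty, and an older spring-arm body chain sits disconnected in the construction script.
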(event `self.ReceiveActorBeginOverlap`
  (params (OtherActor :type "Actor Object Reference"))
  (if (== (`GameplayStatics.GetObjectClass` OtherActor) "/Game/BP/Berry_BP.Berry_BP_C")
    _))

(event `self.ReceiveBeginPlay`
  (bind (_returnvalue_x _returnvalue_y) (`KismetMathLibrary.BreakVector` (`self.K2_GetActorLocation`)))
  (bind _returnvalue (`|SpawnActorFromClass` "/Game/BP/MouseSnakeBody_BP.MouseSnakeBody_BP_C" (`KismetMathLibrary.MakeTransform` (`KismetMathLibrary.MakeVector` _returnvalue_x _returnvalue_y 100.0)) "AlwaysSpawn" "OverrideRootScale" null null))
  (`KismetArrayLibrary.Array_Add` (`self.SnakeBodyArr`) _returnvalue)
  (set `/Game/BP/MouseSnakeBody_BP.Parent` self _returnvalue))

(event `self.ReceiveTick`
  (params (DeltaSeconds :type "Float (single-precision)"))
  (bind (_returnvalue_roll _returnvalue_pitch _returnvalue_yaw) (`KismetMathLibrary.BreakRotator` (`KismetMathLibrary.RInterpTo` (`KismetMathLibrary.FindLookAtRotation` (`self.K2_GetActorLocation`) (`.Location` (`GameplayStatics.BreakHitResult` (`PlayerController.GetHitResultUnderCursorForObjects` (`GameplayStatics.GetPlayerController` 0) (`self.Object Types`) true)))) (`self.K2_GetActorRotation`) (`GameplayStatics.GetWorldDeltaSeconds`) 10.0)))
  (`self.K2_SetActorRotation` (`KismetMathLibrary.MakeRotator` 0.0 0.0 _returnvalue_yaw))
  (`self.AddMovementInput` (`self.DevideVector` (`KismetMathLibrary.GetForwardVector` (`self.K2_GetActorRotation`)) 2.0)))

(fn `DevideVector`
  (params (In :type "Vector Structure") (Coefficient :type "Float (double-precision)"))
  (returns (Return :type "Vector Structure"))
  (locals (Coef_Local :type "Float (double-precision)"))
  (bind _coef_local (`local.Coef_Local`))
  (set `local.Coef_Local` Coefficient)
  (return (`KismetMathLibrary.MakeVector` (/ (.x In) _coef_local) (/ (.y In) _coef_local) (/ (.z In) _coef_local))))

(fn `Set_Tile_BP_ref`
  (`/Engine/EditorBlueprintResources/StandardMacros.IsValid` null
    (:`Is Not Valid`
      (`GameplayStatics.GetActorOfClass` "/Game/BP/Tile_BP.Tile_BP_C"))))

(fn `UserConstructionScript`
  (locals (ParentSpring :type "SpringArmComponent Object Reference") (ParentMesh :type "StaticMeshComponent Object Reference") (XLocation :type "Float (double-precision)") (LagValues :type "Array of Float (double-precision)"))
  (for _ (range 1 21)
    _))