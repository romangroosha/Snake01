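; Player controller that turns W, A, S and D presses into stepped four-direction movement commands.
; Each press calls the MoveCommandPC dispatcher with a fixed-length axis offset and a matching yaw in quarter-turn increments.
; A macro gates all four inputs on a CanMove flag, which a shared tail clears and restores after a short delay as a move cooldown.
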(event `InputAction|W-Action`
  (params (Key :type "Key Structure"))
  (:`Pressed`
    (`self.M_CanMove?`
      (:`true`
        (`self.MoveCommand_PC` (100.0 0.0 0.0))
        (set `self.CanMove?` false :!label _label)
        (`KismetSystemLibrary.Delay` 0.25)
        (set `self.CanMove?` true)))))

(event `InputAction|D-Action`
  (params (Key :type "Key Structure"))
  (:`Pressed`
    (`self.M_CanMove?`
      (:`true`
        (`self.MoveCommand_PC` (0.0 100.0 0.0) (struct :`Yaw` 90.0))
        (goto _label)))))

(event `InputAction|S-Action`
  (params (Key :type "Key Structure"))
  (:`Pressed`
    (`self.M_CanMove?`
      (:`true`
        (`self.MoveCommand_PC` (-100.0 0.0 0.0) (struct :`Yaw` 180.0))
        (goto _label)))))

(event `InputAction|A-Action`
  (params (Key :type "Key Structure"))
  (:`Pressed`
    (`self.M_CanMove?`
      (:`true`
        (`self.MoveCommand_PC` (0.0 -100.0 0.0) (struct :`Yaw` 270.0))
        (goto _label)))))

(fn `UserConstructionScript`)