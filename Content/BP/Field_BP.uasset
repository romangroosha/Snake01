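; Field_BP is an actor that builds a grid play field from tile and barrier actors, sized by X and Y.
; GenerateTile spawns and attaches a Tile_BP per cell at 100-unit spacing, deriving position from a flat index.
; GenerateBarrier repeats the layout for edge-index Barrier_BPs; its mixed X and Y index math assumes a square grid.
; Neither function is called within this Blueprint.
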(fn `GenerateBarrier`
  (bind _output_get (set `self.Total` (* (`self.X`) (`self.Y`))))
  (for _index (range _output_get)
    (if (or (`KismetMathLibrary.InRange_IntInt` _index 0 (- (`self.Y`) 1) false false) (`KismetMathLibrary.InRange_IntInt` _index (- (`self.Total`) (`self.Y`)) (- (`self.Total`) 1) false false) (== (mod _index (`self.X`)) (- (`self.X`) 1)) (== (mod _index (`self.X`)) 0))
      (bind _returnvalue (`|SpawnActorFromClass` "/Game/BP/Barrier_BP.Barrier_BP_C" (`KismetMathLibrary.MakeTransform` (`KismetMathLibrary.MakeVector` (`KismetMathLibrary.Conv_IntToDouble` (* (/ _index (`self.X`)) 100)) (`KismetMathLibrary.Conv_IntToDouble` (* (mod _index (`self.Y`)) 100)))) "Undefined" "OverrideRootScale" null null))
      (`self.K2_AttachToActor` _returnvalue self "None" "KeepRelative" "KeepRelative" "KeepRelative" true))))

(fn `GenerateTile`
  (for _index (range (* (`self.X`) (`self.Y`)))
    (bind _returnvalue (`|SpawnActorFromClass` "/Game/BP/Tile_BP.Tile_BP_C" (`KismetMathLibrary.MakeTransform` (`KismetMathLibrary.MakeVector` (`KismetMathLibrary.Conv_IntToDouble` (* (/ _index (`self.X`)) 100)) (`KismetMathLibrary.Conv_IntToDouble` (* (mod _index (`self.Y`)) 100)))) "Undefined" "OverrideRootScale" null null))
    (`self.K2_AttachToActor` _returnvalue self "None" "KeepRelative" "KeepRelative" "KeepRelative" true)))

(fn `UserConstructionScript`)