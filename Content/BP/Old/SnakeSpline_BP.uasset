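; Snake actor that moves in steps on player controller commands and records its path in a separately spawned Spline_BP.
; Each move command rotates the Sphere, appends the offset position to SnakeMoves, adds it as a linear spline point and teleports the actor there.
; The N key is a debug hook that prints the stored moves and updates the spline.
; Spline rebuild and spline-mesh generation logic is present but disconnected.
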(event `self.ReceiveBeginPlay`
  (bind _returnvalue (`self.GetTransform`))
  (`self.GameModeBase_BP_ref`)
  (`self.PlayerController_BP_ref`)
  (add `/Game/BP/PlayerController_BP.MoveCommand_PC` (`self.PlayerController_BP`) (`|CreateDelegate` :!event `MoveCommand_PC`))
  (bind _returnvalue_2 (`|SpawnActorFromClass` "/Game/BP/Old/Spline_BP.Spline_BP_C" (`KismetMathLibrary.MakeTransform` (`KismetMathLibrary.MakeVector` (.x (.location _returnvalue)) (.y (.location _returnvalue))) (.rotation _returnvalue) (.scale _returnvalue)) "Undefined" "OverrideRootScale" null null))
  (set `self.Spline_BP` _returnvalue_2)
  (`KismetArrayLibrary.Array_Add` (`self.SnakeMoves`) (`self.K2_GetActorLocation`))
  (`KismetArrayLibrary.Array_Add` (`self.SnakeMoves`) (`self.K2_GetActorLocation`)))

(event `MoveCommand_PC`
  (params (Location :type "Vector Structure") (Rotation :type "Rotator Structure"))
  (bind _snakemoves (`self.SnakeMoves`))
  (`SceneComponent.K2_SetWorldRotation` (`self.Sphere`) Rotation false true)
  (bind _returnvalue (`KismetArrayLibrary.Array_Add` _snakemoves (+ Location (`self.K2_GetActorLocation`))))
  (bind _output (`|GetArrayItem` _snakemoves _returnvalue))
  (`SplineComponent.AddPoint` (`/Game/BP/Old/Spline_BP.Spline` (`self.Spline_BP`)) (make `SplinePoint` (`KismetMathLibrary.Conv_IntToDouble` _returnvalue) _output (0.0 0.0 0.0) (0.0 0.0 0.0) (struct) (1.0 1.0 1.0) "Linear") true)
  (`self.K2_SetActorLocation` _output false true))

(event `Key|N`
  (params (Key :type "Key Structure"))
  (:`Pressed`
    (for _array_element (`self.SnakeMoves`)
      (`/Game/BP/MacroLibrary.Print Red String` (`KismetStringLibrary.Conv_VectorToString` _array_element))
      (`SplineComponent.UpdateSpline` (`/Game/BP/Old/Spline_BP.Spline` (`self.Spline_BP`))))))

(fn `GameModeBase_BP_ref`
  (`/Engine/EditorBlueprintResources/StandardMacros.IsValid` (`self.GameModeBase_BP`)
    (:`Is Not Valid`
      (bind _returnvalue (`GameplayStatics.GetActorOfClass` "/Game/BP/GameModeBase_BP.GameModeBase_BP_C"))
      (set `self.GameModeBase_BP` _returnvalue))))

(fn `PlayerController_BP_ref`
  (`/Engine/EditorBlueprintResources/StandardMacros.IsValid` (`self.PlayerController_BP`)
    (:`Is Not Valid`
      (bind _returnvalue (`GameplayStatics.GetActorOfClass` "/Game/BP/PlayerController_BP.PlayerController_BP_C"))
      (set `self.PlayerController_BP` _returnvalue))))

(fn `UserConstructionScript`)