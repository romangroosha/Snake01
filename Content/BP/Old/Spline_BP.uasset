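; Spline actor that builds spline mesh segments along its Spline when the player controller broadcasts a move command.
; BeginPlay caches PlayerController_BP and binds to its MoveCommand_PC dispatcher.
; Each command adds one mesh per SectionLength step, with tangents clamped to that length, ignoring Location and Rotation and never clearing earlier segments.
; A duplicate of the build loop sits disconnected in the construction script.
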(event `self.ReceiveBeginPlay`
  (`self.PlayerController_BP_ref`)
  (add `/Game/BP/PlayerController_BP.MoveCommand_PC` (`self.PlayerController_BP`) (`|CreateDelegate` :!event `MoveCommand_PC`)))

(event `MoveCommand_PC`
  (params (Location :type "Vector Structure") (Rotation :type "Rotator Structure"))
  (for _index (range (+ (`KismetMathLibrary.FTrunc` (/ (`SplineComponent.GetSplineLength` (`self.Spline`)) (`self.SectionLength`))) 1))
    (bind _returnvalue (`AddComponent|NODE_AddSplineMeshComponent-1`))
    (`SplineMeshComponent.SetForwardAxis` _returnvalue "X" true)
    (bind _returnvalue_2 (* _index (`self.SectionLength`)))
    (bind _returnvalue_3 (* (+ _index 1) (`self.SectionLength`)))
    (`SplineMeshComponent.SetStartAndEnd` _returnvalue (`SplineComponent.GetLocationAtDistanceAlongSpline` (`self.Spline`) _returnvalue_2 "Local") (`KismetMathLibrary.ClampVectorSize` (`SplineComponent.GetTangentAtDistanceAlongSpline` (`self.Spline`) _returnvalue_2 "Local") 0.0 (`self.SectionLength`)) (`SplineComponent.GetLocationAtDistanceAlongSpline` (`self.Spline`) _returnvalue_3 "Local") (`KismetMathLibrary.ClampVectorSize` (`SplineComponent.GetTangentAtDistanceAlongSpline` (`self.Spline`) _returnvalue_3 "Local") 0.0 (`self.SectionLength`)) true)))

(fn `PlayerController_BP_ref`
  (`/Engine/EditorBlueprintResources/StandardMacros.IsValid` (`self.PlayerController_BP`)
    (:`Is Not Valid`
      (bind _returnvalue (`GameplayStatics.GetActorOfClass` "/Game/BP/PlayerController_BP.PlayerController_BP_C"))
      (set `self.PlayerController_BP` _returnvalue))))

(fn `UserConstructionScript`)