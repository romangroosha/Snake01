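; Body segment of the mouse-controlled snake that trails the actor ahead of it and can grow the tail.
; Each tick it interpolates its location and rotation toward its Parent, forming a follow-the-leader chain.
; The Berryable interface event spawns a new segment at the Sphere's X/Y, adds it to MouseSnake_BP's body array and parents it to itself.
; Spring arm tuning from the game mode is present but never runs.
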(event `self.ReceiveBeginPlay`
  (`self.Set_MouseSnakeBP_ref`)
  (`self.GameModeBase_BP_ref`))

(event `/Game/BP/Berryable_INT.Berryable_Interface`
  (bind (_returnvalue_x _returnvalue_y) (`KismetMathLibrary.BreakVector` (`SceneComponent.K2_GetComponentLocation` (`self.Sphere`))))
  (bind _returnvalue (`|SpawnActorFromClass` "MouseSnakeBody_BP_C" (`KismetMathLibrary.MakeTransform` (`KismetMathLibrary.MakeVector` _returnvalue_x _returnvalue_y)) "AlwaysSpawn" "OverrideRootScale" null null))
  (`KismetArrayLibrary.Array_Add` (`/Game/BP/MouseSnake_BP.SnakeBodyArr` (`self.MouseSnakeBP_ref`)) _returnvalue)
  (set `/Game/BP/MouseSnakeBody_BP.Parent` self _returnvalue))

(event `self.ReceiveTick`
  (params (DeltaSeconds :type "Float (single-precision)"))
  (`self.UpdateLocRot` 10.0))

(fn `GameModeBase_BP_ref`
  (`/Engine/EditorBlueprintResources/StandardMacros.IsValid` (`self.GameModeBase_BP`)
    (:`Is Not Valid`
      (bind _returnvalue (`GameplayStatics.GetActorOfClass` "/Game/BP/GameModeBase_BP.GameModeBase_BP_C"))
      (set `self.GameModeBase_BP` _returnvalue))))

(fn `Set_MouseSnakeBP_ref`
  (`/Engine/EditorBlueprintResources/StandardMacros.IsValid` (`self.MouseSnakeBP_ref`)
    (:`Is Not Valid`
      (bind _returnvalue (`GameplayStatics.GetActorOfClass` "/Game/BP/MouseSnake_BP.MouseSnake_BP_C"))
      (set `self.MouseSnakeBP_ref` _returnvalue))))

(fn `UpdateLocRot`
  (params (`Location Delay` :type "Float (single-precision)" :default 10.0) (`Rotation Delay` :type "Float (single-precision)" :default 10.0))
  (`self.K2_SetActorLocation` (`KismetMathLibrary.VInterpTo` (`self.K2_GetActorLocation`) (`self.K2_GetActorLocation` (`self.Parent`)) (`GameplayStatics.GetWorldDeltaSeconds`) `Location Delay`))
  (`self.K2_SetActorRotation` (`KismetMathLibrary.RInterpTo` (`self.K2_GetActorRotation`) (`self.K2_GetActorRotation` (`self.Parent`)) (`GameplayStatics.GetWorldDeltaSeconds`) `Rotation Delay`)))

(fn `UserConstructionScript`)