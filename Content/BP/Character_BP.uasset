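; Snake-style head Character that moves in steps and pauses the game on hitting a barrier or any body segment except the first.
; BeginPlay caches GameMode and PlayerController, binds their move dispatchers, and spawns the first Body_BP behind it.
; Each controller move command rotates the head mesh and lerps the actor by the given offset, using a timeline rate derived from the GameMode's tick interval.
; The ticker, berry interface and Tick handlers are empty.
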(event `MoveTicker_Event`)

(event `self.ReceiveBeginPlay`
  (bind (_actorlocationba_x _actorlocationba_y) (`KismetMathLibrary.BreakVector` (`self.ActorLocationBA`)))
  (`self.GameModeBase_BP_ref`)
  (`self.PlayerController_BP_ref`)
  (add `/Game/BP/PlayerController_BP.MoveCommand_PC` (`self.PlayerController_BP`) (`|CreateDelegate` :!event `MoveCommand_PC`))
  (add `/Game/BP/GameModeBase_BP.MoveTicker` (`self.GameModeBase_BP`) (`|CreateDelegate` :!event `MoveTicker_Event`))
  (set `self.ActorLocationBA` (`self.K2_GetActorLocation`))
  (`TimelineComponent.SetPlayRate` (`self.Timeline_1`) (/ 1.0 (`/Game/BP/GameModeBase_BP.TimeRate (in seconds)` (`self.GameModeBase_BP`))))
  (bind _returnvalue (`|SpawnActorFromClass` "/Game/BP/Body_BP.Body_BP_C" (`KismetMathLibrary.MakeTransform` (`KismetMathLibrary.MakeVector` _actorlocationba_x (+ _actorlocationba_y -100.0))) "Undefined" "OverrideRootScale" null null))
  (set `/Game/BP/Body_BP.ParentAct` self _returnvalue)
  (`KismetArrayLibrary.Array_Add` (`self.BodyArr`) _returnvalue))

(event `MoveCommand_PC`
  (params (Location :type "Vector Structure") (Rotation :type "Rotator Structure"))
  (set `self.DirectionBA` Location)
  (set `self.ActorLocationBA` (`self.K2_GetActorLocation`))
  (bind _output_get (set `self.HeadRotationBA` Rotation))
  (`SceneComponent.K2_SetWorldRotation` (`self.Cube`) _output_get false true)
  (bind (_direction _0_to_1) (`Timeline|Timeline_1` :!via `PlayFromStart`)
    (:`Update`
      (`self.K2_SetActorLocation` (`KismetMathLibrary.VLerp` (`self.ActorLocationBA`) (+ (`self.ActorLocationBA`) (`self.DirectionBA`)) _0_to_1) false true))
    (:`Finished`)))

(event `/Game/BP/Berryable_INT.Berryable_Interface`)

(event `self.CapsuleComponent.OnComponentBeginOverlap`
  (params (OverlappedComponent :type "PrimitiveComponent Object Reference") (OtherActor :type "Actor Object Reference") (OtherComp :type "PrimitiveComponent Object Reference") (OtherBodyIndex :type Integer) (bFromSweep :type Boolean) (SweepResult :type "HitResult Structure (by ref)"))
  (bind _returnvalue (`GameplayStatics.GetObjectClass` OtherActor))
  (if (or (== _returnvalue "/Game/BP/Barrier_BP.Barrier_BP_C") (and (== _returnvalue "/Game/BP/Body_BP.Body_BP_C") (!= OtherActor (`|GetArrayItem` (`self.BodyArr`)))))
    (`StaticMeshComponent.SetStaticMesh` (`self.Cone`) "/Engine/EngineMeshes/Cube.Cube")
    (`SceneComponent.SetWorldScale3D` (`self.Cone`) (0.35 0.35 0.35))
    (`GameplayStatics.SetGamePaused` true)))

(event `self.ReceiveActorBeginOverlap`
  (params (OtherActor :type "Actor Object Reference")))

(event `self.ReceiveTick`
  (params (DeltaSeconds :type "Float (single-precision)")))

(fn `GameModeBase_BP_ref`
  (`/Engine/EditorBlueprintResources/StandardMacros.IsValid` (`self.GameModeBase_BP`)
    (:`Is Not Valid`
      (bind _returnvalue (`GameplayStatics.GetActorOfClass` "/Game/BP/GameModeBase_BP.GameModeBase_BP_C"))
      (set `self.GameModeBase_BP` _returnvalue))))

(fn `PlayerController_BP_ref`
  (`/Engine/EditorBlueprintResources/StandardMacros.IsValid` (`self.PlayerController_BP`)
    (:`Is Not Valid`
      (bind _returnvalue (`GameplayStatics.GetActorOfClass` "/Game/BP/PlayerController_BP.PlayerController_BP_C"))
      (set `self.PlayerController_BP` _returnvalue))))

(fn `UserConstructionScript`)